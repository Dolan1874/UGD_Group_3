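; BP_Interactable_BlockPickup is an interactable pickup that gives the top-down character a block.
; On Interact it prints the interactor's name, casts it to BP_TopDownCharacter, sets its HasBlock flag, prints a confirmation and destroys itself.
; CanInteract defers to the parent, and GetInteractText returns an empty string.
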(event `/Game/UGD_Game/Interfaces/BPI_Interactable.Interact`
  (params (Interactor :type "Actor Object Reference"))
  (`KismetSystemLibrary.PrintString` (`KismetStringLibrary.Concat_StrStr` "This is name of class " (`KismetSystemLibrary.GetDisplayName` Interactor)))
  (bind _asbp_top_down_character (cast `/Game/UGD_Game/Blueprints/BP_TopDownCharacter` Interactor))
  (set `/Game/UGD_Game/Blueprints/BP_TopDownCharacter.HasBlock` true _asbp_top_down_character)
  (`KismetSystemLibrary.PrintString` "Picked up block")
  (`self.K2_DestroyActor`))

(fn `CanInteract`
  (returns (IsInteractable :type Boolean))
  (bind _isinteractable (`parent.CanInteract`))
  (return _isinteractable))

(fn `GetInteractText`
  (returns (TextPrompt :type Text))
  (return ""))

(fn `UserConstructionScript`
  (`parent.UserConstructionScript`))