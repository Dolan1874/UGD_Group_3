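; Interactable coloured block pickup that flags the interacting character as holding a block, then destroys itself.
; A BlockID enum selects the mesh material on BeginPlay, and ApplyIDandColour lets callers change the ID and refresh the colour.
; Interact casts to UGD_Character, falling back to BP_TopDownCharacter with a debug class-name print.
; Pickup sets only HasBlock on the character, so the BlockID is not handed over.
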(event `self.ReceiveBeginPlay`
  (`self.ApplyBlockColour`))

(event `/Game/UGD_Game/Interfaces/BPI_Interactable.Interact`
  (params (Interactor :type "Actor Object Reference"))
  (bind _asugd_character (cast `/Game/UGD_Game/Blueprints/NPC_Stuff/UGD_Character` Interactor)
    (:`then`
      (set `/Game/UGD_Game/Blueprints/NPC_Stuff/UGD_Character.HasBlock` true _asugd_character))
    (:`CastFailed`
      (`KismetSystemLibrary.PrintString` (`KismetStringLibrary.Concat_StrStr` "This is name of class " (`KismetSystemLibrary.GetDisplayName` Interactor)))
      (bind _asbp_top_down_character (cast `/Game/UGD_Game/Blueprints/BP_TopDownCharacter` Interactor))
      (set `/Game/UGD_Game/Blueprints/BP_TopDownCharacter.HasBlock` true _asbp_top_down_character)))
  (`KismetSystemLibrary.PrintString` "Picked up block")
  (`self.K2_DestroyActor`))

(fn `ApplyBlockColour`
  (switch `/Game/UGD_Game/Blueprints/BlockID_E` (`self.BlockID`)
    (:`NewEnumerator1`
      (`PrimitiveComponent.SetMaterial` (`self.Mesh`) 0 "/Game/LevelPrototyping/Materials/Colours/M_Red.M_Red"))
    (:`NewEnumerator2`
      (`PrimitiveComponent.SetMaterial` (`self.Mesh`) 0 "/Game/LevelPrototyping/Materials/Colours/M_Yellow.M_Yellow"))
    (:`NewEnumerator3`
      (`PrimitiveComponent.SetMaterial` (`self.Mesh`) 0 "/Game/LevelPrototyping/Materials/Colours/M_Blue.M_Blue"))
    (:`NewEnumerator4`
      (`PrimitiveComponent.SetMaterial` (`self.Mesh`) 0 "/Game/LevelPrototyping/Materials/Colours/M_Green.M_Green"))
    (:`NewEnumerator5`
      (`PrimitiveComponent.SetMaterial` (`self.Mesh`) 0 "/Game/LevelPrototyping/Materials/Colours/M_Purple.M_Purple"))
    (:`NewEnumerator6`
      (`PrimitiveComponent.SetMaterial` (`self.Mesh`) 0 "/Game/LevelPrototyping/Materials/Colours/M_Orange.M_Orange"))
    (:`NewEnumerator7`
      (`PrimitiveComponent.SetMaterial` (`self.Mesh`) 0 "/Game/LevelPrototyping/Materials/Colours/M_White.M_White"))
    (:`NewEnumerator8`
      (`PrimitiveComponent.SetMaterial` (`self.Mesh`) 0 "/Game/LevelPrototyping/Materials/Colours/M_Black.M_Black"))))

(fn `ApplyIDandColour`
  (params (NewBlockID :type "/Game/UGD_Game/Blueprints/BlockID_E Enum" :default "NewEnumerator0"))
  (set `self.BlockID` NewBlockID)
  (`self.ApplyBlockColour`))

(fn `CanInteract`
  (returns (IsInteractable :type Boolean))
  (bind _isinteractable (`parent.CanInteract`))
  (return _isinteractable))

(fn `GetInteractText`
  (returns (TextPrompt :type Text))
  (return ""))

(fn `UserConstructionScript`
  (`parent.UserConstructionScript`))