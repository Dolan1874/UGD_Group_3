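; Colour-coded puzzle button that activates a linked target object, such as a door, when a matching block is placed on it.
; BeginPlay sets the button face material from its BlockID enum.
; Box overlap compares the block's ID with its own, then calls Activate on TargetObj through activatable_object_parent_BP.
; End overlap calls Deactivate whenever IsBlock is set, without checking which actor left.
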(event `self.ReceiveBeginPlay`
  ; changes button colour depending on enum
  (`self.Get colour`))

(event `self.Box.OnComponentBeginOverlap`
  (params (OverlappedComponent :type "PrimitiveComponent Object Reference") (OtherActor :type "Actor Object Reference") (OtherComp :type "PrimitiveComponent Object Reference") (OtherBodyIndex :type Integer) (bFromSweep :type Boolean) (SweepResult :type "HitResult Structure (by ref)"))
  ; opens target door when the right block is placed on the button
  (bind _asbp_interactable_block_pickup (cast `/Game/UGD_Game/Blueprints/migrated_block/BP_Interactable_BlockPickup` OtherActor)
    (:`then`
      (bind _output_get (set `self.collision_ID` (`/Game/UGD_Game/Blueprints/migrated_block/BP_Interactable_BlockPickup.BlockID` _asbp_interactable_block_pickup)))
      (if (`KismetStringLibrary.EqualEqual_StrStr` (`|GetEnumeratorNameAsString` _output_get) (`|GetEnumeratorNameAsString` (`self.block_ID`)))
        (set `self.is block` true)
        (bind _asactivatable_object_parent_bp (cast `/Game/UGD_Game/Blueprints/activatable_object_parent_BP` (`self.target_obj`))
          (:`then`
            (`/Game/UGD_Game/Blueprints/activatable_object_parent_BP.activate` _asactivatable_object_parent_bp))
          (:`CastFailed`
            (`KismetSystemLibrary.PrintString` "no target")))
        (else
          (`KismetSystemLibrary.PrintString` "blocks dont match"))))
    (:`CastFailed`
      (`KismetSystemLibrary.PrintString` "not a block"))))

(event `self.Box.OnComponentEndOverlap`
  (params (OverlappedComponent :type "PrimitiveComponent Object Reference") (OtherActor :type "Actor Object Reference") (OtherComp :type "PrimitiveComponent Object Reference") (OtherBodyIndex :type Integer))
  ; closes door when block is removed from the button
  (if (`self.is block`)
    (set `self.is block` false)
    (bind _asactivatable_object_parent_bp (cast `/Game/UGD_Game/Blueprints/activatable_object_parent_BP` (`self.target_obj`))
      (:`then`
        (`/Game/UGD_Game/Blueprints/activatable_object_parent_BP.Deactivate` _asactivatable_object_parent_bp))
      (:`CastFailed`
        (`KismetSystemLibrary.PrintString` "no target")))
    (else
      (`KismetSystemLibrary.PrintString` "wasnt a block"))))

(fn `Get colour`
  (switch `/Game/UGD_Game/Blueprints/BlockID_E` (`self.block_ID`)
    (:`NewEnumerator1`
      (`PrimitiveComponent.SetMaterial` (`self.Button face`) 0 "/Game/LevelPrototyping/Materials/Colours/M_Red.M_Red"))
    (:`NewEnumerator2`
      (`PrimitiveComponent.SetMaterial` (`self.Button face`) 0 "/Game/LevelPrototyping/Materials/Colours/M_Yellow.M_Yellow"))
    (:`NewEnumerator3`
      (`PrimitiveComponent.SetMaterial` (`self.Button face`) 0 "/Game/LevelPrototyping/Materials/Colours/M_Blue.M_Blue"))
    (:`NewEnumerator4`
      (`PrimitiveComponent.SetMaterial` (`self.Button face`) 0 "/Game/LevelPrototyping/Materials/Colours/M_Green.M_Green"))
    (:`NewEnumerator5`
      (`PrimitiveComponent.SetMaterial` (`self.Button face`) 0 "/Game/LevelPrototyping/Materials/Colours/M_Purple.M_Purple"))
    (:`NewEnumerator6`
      (`PrimitiveComponent.SetMaterial` (`self.Button face`) 0 "/Game/LevelPrototyping/Materials/Colours/M_Orange.M_Orange"))
    (:`NewEnumerator7`
      (`PrimitiveComponent.SetMaterial` (`self.Button face`) 0 "/Game/LevelPrototyping/Materials/Colours/M_White.M_White"))
    (:`NewEnumerator8`
      (`PrimitiveComponent.SetMaterial` (`self.Button face`) 0 "/Game/LevelPrototyping/Materials/Colours/M_Black.M_Black"))))

(fn `UserConstructionScript`)