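; Keypad actor that controls a linked Door and shows its activation progress through its material colour.
; It extends parent trigger, activate and deactivate logic: triggering opens the door only when activated, and deactivating closes it.
; Activation changes refresh the keypad to red, yellow or green based on how many of its required buttons are active.
; Keycard handling only prints debug messages.
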(fn `activate`
  (`parent.activate`)
  (`self.change colour`))

(fn `change colour`
  ; change keypad colour depending on if its complete or prtialy complete
  (if (> (`self.activated buttons`) 0)
    (if (== (`self.activated buttons`) (`self.total buttons`))
      (`PrimitiveComponent.SetMaterial` (`self.keypad`) 0 "/Game/UGD_Game/Materials/Colours/M_Green.M_Green")
      (else
        (`PrimitiveComponent.SetMaterial` (`self.keypad`) 0 "/Game/UGD_Game/Materials/Colours/M_Yellow.M_Yellow")))
    (else
      (`PrimitiveComponent.SetMaterial` (`self.keypad`) 0 "/Game/UGD_Game/Materials/Colours/M_Red.M_Red"))))

(fn `Deactivate`
  (`parent.Deactivate`)
  (`self.change colour`)
  (bind _asdoor (cast `/Game/UGD_Game/Blueprints/Door` (`self.door`))
    (:`then`
      (`/Game/UGD_Game/Blueprints/Door.close` _asdoor))
    (:`CastFailed`
      (`KismetSystemLibrary.PrintString` "no door"))))

(fn `trigger`
  (`parent.trigger`)
  (if (`self.activated`)
    (bind _asdoor (cast `/Game/UGD_Game/Blueprints/Door` (`self.door`))
      (:`then`
        (`/Game/UGD_Game/Blueprints/Door.open` _asdoor))
      (:`CastFailed`
        (`KismetSystemLibrary.PrintString` "no door")))
    (else
      (`KismetSystemLibrary.PrintString` "door cant open"))))

(fn `UseKeyCard`
  (params (KeycardColour :type "/Game/UGD_Game/Blueprints/Block_Stuff/BlockID_E Enum" :default "NewEnumerator0"))
  (switch `/Game/UGD_Game/Blueprints/Block_Stuff/BlockID_E` KeycardColour
    (:`NewEnumerator0`
      (`KismetSystemLibrary.PrintString` "keycard received none"))
    (:`NewEnumerator1`
      (`KismetSystemLibrary.PrintString` "Keycard received red"))))

(fn `UserConstructionScript`
  (`parent.UserConstructionScript`))