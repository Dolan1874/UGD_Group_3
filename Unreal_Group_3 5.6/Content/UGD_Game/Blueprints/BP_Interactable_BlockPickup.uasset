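; Interactable coloured block pickup that characters collect, destroying the actor on pickup.
; On BeginPlay it sets its mesh material from BlockID and registers as an AI sight stimulus so NPCs can see it; ApplyIDandColour changes both ID and colour.
; Interact flags HasBlock on a UGD_Character, or stores the ID on a BP_TopDownCharacter and adds the block, with its world class, to that character's inventory.
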(event `self.ReceiveBeginPlay`
  (`|ExecutionSequence`
    (:`then_0`
      ; Apply the colours to the block
      (`self.ApplyBlockColourID`))
    (:`then_1`
      ; Registers the block as a perception stimuli source so the NPC can see it
      (`AIPerceptionSystem.RegisterPerceptionStimuliSource` "/Script/AIModule.AISense_Sight" self))))

(event `/Game/UGD_Game/Interfaces/BPI_Interactable.Interact`
  (params (Interactor :type "Actor Object Reference"))
  (bind _asugd_character (cast `/Game/UGD_Game/Blueprints/NPC_Stuff/UGD_Character` Interactor)
    (:`then`
      (set `/Game/UGD_Game/Blueprints/NPC_Stuff/UGD_Character.HasBlock` true _asugd_character)
      (`KismetSystemLibrary.PrintString` "Picked up block" :!label _label)
      (`self.K2_DestroyActor`))
    (:`CastFailed`
      (bind _asbp_top_down_character (cast `/Game/UGD_Game/Blueprints/BP_TopDownCharacter` Interactor)
        (:`then`
          (bind _output_get (set `/Game/UGD_Game/Blueprints/BP_TopDownCharacter.HeldBlockID` (`self.BlockID`) _asbp_top_down_character))
          (`/Game/UGD_Game/Blueprints/BP_InventoryComponent.AddItemToInventory` (`/Game/UGD_Game/Blueprints/BP_TopDownCharacter.BP_InventoryComponent` _asbp_top_down_character) "NewEnumerator1" _output_get null "/Game/UGD_Game/Blueprints/migrated_block/BP_Interactable_BlockPickup.BP_Interactable_BlockPickup_C")
          (goto _label))
        (:`CastFailed`
          (`KismetSystemLibrary.PrintString` "Cast to TopDownCharacter failed in Block Pickup"))))))

(fn `ApplyBlockColourID`
  (switch `/Game/UGD_Game/Blueprints/BlockID_E` (`self.BlockID`)
    (:`NewEnumerator1`
      (`PrimitiveComponent.SetMaterial` (`self.Mesh`) 0 "/Game/UGD_Game/Materials/Colours/M_Red.M_Red"))
    (:`NewEnumerator2`
      (`PrimitiveComponent.SetMaterial` (`self.Mesh`) 0 "/Game/UGD_Game/Materials/Colours/M_Yellow.M_Yellow"))
    (:`NewEnumerator3`
      (`PrimitiveComponent.SetMaterial` (`self.Mesh`) 0 "/Game/UGD_Game/Materials/Colours/M_Blue.M_Blue"))
    (:`NewEnumerator4`
      (`PrimitiveComponent.SetMaterial` (`self.Mesh`) 0 "/Game/UGD_Game/Materials/Colours/M_Green.M_Green"))
    (:`NewEnumerator5`
      (`PrimitiveComponent.SetMaterial` (`self.Mesh`) 0 "/Game/UGD_Game/Materials/Colours/M_Purple.M_Purple"))
    (:`NewEnumerator6`
      (`PrimitiveComponent.SetMaterial` (`self.Mesh`) 0 "/Game/UGD_Game/Materials/Colours/M_Orange.M_Orange"))
    (:`NewEnumerator7`
      (`PrimitiveComponent.SetMaterial` (`self.Mesh`) 0 "/Game/UGD_Game/Materials/Colours/M_White.M_White"))
    (:`NewEnumerator8`
      (`PrimitiveComponent.SetMaterial` (`self.Mesh`) 0 "/Game/UGD_Game/Materials/Colours/M_Black.M_Black"))))

(fn `ApplyIDandColour`
  (params (`New Block ID` :type "/Game/UGD_Game/Blueprints/BlockID_E Enum" :default "NewEnumerator0"))
  (set `self.BlockID` `New Block ID`)
  (`self.ApplyBlockColourID`))

(fn `CanInteract`
  (returns (IsInteractable :type Boolean))
  (bind _isinteractable (`parent.CanInteract`))
  (return _isinteractable))

(fn `GetInteractText`
  (returns (TextPrompt :type Text))
  (return ""))

(fn `UserConstructionScript`
  (`parent.UserConstructionScript`))