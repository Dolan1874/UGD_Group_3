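; Inventory component that stores picked items in a small fixed-size array of slot structs.
; BeginPlay clears the array and fills it with empty, unoccupied slots.
; AddItemToInventory writes item type, block ID, icon and world class into the first free slot, then stops; a full inventory silently ignores the item.
; A switch on the stored block ID's color follows each write, but all its branches are empty.
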(event `self.ReceiveBeginPlay`
  (`KismetArrayLibrary.Array_Clear` (`self.InventorySlots`))
  (for _ (range 5)
    (`KismetArrayLibrary.Array_Add` (`self.InventorySlots`) (make `/Game/UGD_Game/Blueprints/Inventory_Stuff/S_InventorySlot` false "NewEnumerator0" "NewEnumerator0" null))))

(fn `AddItemToInventory`
  (params (ItemType :type "/Game/UGD_Game/Blueprints/Inventory_Stuff/ItemType_E Enum" :default "NewEnumerator0") (BlockID :type "/Game/UGD_Game/Blueprints/Block_Stuff/BlockID_E Enum" :default "NewEnumerator0") (ItemIcon :type "Texture2D Object Reference") (WorldClass :type "Actor Class Reference"))
  (for _index (range 5)
    (if (not (`.Occupied_2_CCB9DE3E414440BCFABB19B2E966F4DC` (break `/Game/UGD_Game/Blueprints/Inventory_Stuff/S_InventorySlot` (`|GetArrayItem` (`self.InventorySlots`) _index))))
      (`KismetArrayLibrary.Array_Set` (`self.InventorySlots`) _index (make `/Game/UGD_Game/Blueprints/Inventory_Stuff/S_InventorySlot` true ItemType BlockID ItemIcon WorldClass))
      (switch `/Game/UGD_Game/Blueprints/Block_Stuff/BlockID_E` (`.BlockID_7_16B677134CB6E3D059AC15834D252343` (break `/Game/UGD_Game/Blueprints/Inventory_Stuff/S_InventorySlot` (`|GetArrayItem` (`self.InventorySlots`) _index)))
        (:`NewEnumerator0`
          _)
        (:`NewEnumerator1`
          _)
        (:`NewEnumerator2`
          _)
        (:`NewEnumerator3`
          _)
        (:`NewEnumerator4`
          _)
        (:`NewEnumerator5`
          _)
        (:`NewEnumerator6`
          _)
        (:`NewEnumerator7`
          _)
        (:`NewEnumerator8`
          _))
      (return))))