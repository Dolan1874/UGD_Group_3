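; Interactable keycard pickup that adds a colour-coded keycard to the top-down character's inventory.
; On BeginPlay it sets the mesh material from its BlockID colour, so the construction script does not apply the colour.
; Its HandleInteract override skips the parent, adds the item with its ID, icon and class to the interactor's inventory component, refreshes the inventory widget, then destroys the actor.
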(event `self.ReceiveBeginPlay`
  (`self.ApplyKeycardColour`))

(fn `ApplyKeycardColour`
  (switch `/Game/UGD_Game/Blueprints/Block_Stuff/BlockID_E` (`self.BlockID`)
    (:`NewEnumerator1`
      (`PrimitiveComponent.SetMaterial` (`self.Mesh`) 0 (`self.RedMat`)))
    (:`NewEnumerator2`
      (`PrimitiveComponent.SetMaterial` (`self.Mesh`) 0 (`self.YellowMat`)))
    (:`NewEnumerator3`
      (`PrimitiveComponent.SetMaterial` (`self.Mesh`) 0 (`self.BlueMat`)))
    (:`NewEnumerator4`
      (`PrimitiveComponent.SetMaterial` (`self.Mesh`) 0 (`self.GreenMat`)))
    (:`NewEnumerator5`
      (`PrimitiveComponent.SetMaterial` (`self.Mesh`) 0 (`self.PurpleMat`)))
    (:`NewEnumerator6`
      (`PrimitiveComponent.SetMaterial` (`self.Mesh`) 0 (`self.OrangeMat`)))
    (:`NewEnumerator7`
      (`PrimitiveComponent.SetMaterial` (`self.Mesh`) 0 (`self.WhiteMat`)))
    (:`NewEnumerator8`
      (`PrimitiveComponent.SetMaterial` (`self.Mesh`) 0 (`self.BlackMat`)))))

(fn `HandleInteract`
  (params (Interactor :type "Actor Object Reference"))
  (bind _asbp_top_down_character (cast `/Game/UGD_Game/Blueprints/BP_TopDownCharacter` Interactor))
  (`/Game/UGD_Game/Blueprints/Inventory_Stuff/BP_InventoryComponent.AddItemToInventory` (`/Game/UGD_Game/Blueprints/BP_TopDownCharacter.BP_InventoryComponent` _asbp_top_down_character) "NewEnumerator2" (`self.BlockID`) (`self.ItemIcon`) "BP_Interactable_KeycardPickup_C")
  (`/Game/UGD_Game/Blueprints/BP_TopDownCharacter.RefreshInventoryWidget` _asbp_top_down_character)
  (`KismetSystemLibrary.PrintString` "Picked up keycard")
  (`self.K2_DestroyActor`))

(fn `UserConstructionScript`
  (`parent.UserConstructionScript`))