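; Colour-coded pressure button that activates a target object, such as a door, when a matching pickup block rests on it.
; BeginPlay sets the face material from the BlockID colour enum.
; Box overlap compares the block's ID to the button's, then lowers the face and calls Activate on TargetObj through activatable_object_parent_BP.
; End overlap raises it and calls Deactivate if pressed, without checking which actor left.
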(event `self.ReceiveBeginPlay`
  ; changes button colour depending on enum
  (`self.Get colour`))

(event `self.Box.OnComponentBeginOverlap`
  (params (OverlappedComponent :type "PrimitiveComponent Object Reference") (OtherActor :type "Actor Object Reference") (OtherComp :type "PrimitiveComponent Object Reference") (OtherBodyIndex :type Integer) (bFromSweep :type Boolean) (SweepResult :type "HitResult Structure (by ref)"))
  ; opens target door when the right block is placed on the button
  (bind _asbp_interactable_block_pickup (cast `/Game/UGD_Game/Blueprints/Block_Stuff/BP_Interactable_BlockPickup` OtherActor)
    (:`then`
      (bind _output_get (set `self.collision_ID` (cast `/Game/UGD_Game/Blueprints/Block_Stuff/BlockID_E` (`/Game/UGD_Game/Blueprints/Block_Stuff/BP_Interactable_BlockPickup.BlockID` _asbp_interactable_block_pickup))))
      (if (`KismetStringLibrary.EqualEqual_StrStr` (`|GetEnumeratorNameAsString` _output_get) (`|GetEnumeratorNameAsString` (`self.block_ID`)))
        (set `self.is block` true)
        (`SceneComponent.K2_AddLocalOffset` (`self.Button face`) (0.0 0.0 -3.0) false false)
        (bind _asactivatable_object_parent_bp (cast `/Game/UGD_Game/Blueprints/activatable_object_parent_BP` (`self.target_obj`))
          (:`then`
            (`/Game/UGD_Game/Blueprints/activatable_object_parent_BP.activate` _asactivatable_object_parent_bp))
          (:`CastFailed`
            (`KismetSystemLibrary.PrintString` "no target")))
        (else
          (`KismetSystemLibrary.PrintString` "blocks dont match"))))
    (:`CastFailed`
      (`KismetSystemLibrary.PrintString` "not a block"))))

(event `self.Box.OnComponentEndOverlap`
  (params (OverlappedComponent :type "PrimitiveComponent Object Reference") (OtherActor :type "Actor Object Reference") (OtherComp :type "PrimitiveComponent Object Reference") (OtherBodyIndex :type Integer))
  ; closes door when block is removed from the button
  (if (`self.is block`)
    (set `self.is block` false)
    (`SceneComponent.K2_AddLocalOffset` (`self.Button face`) (0.0 0.0 3.0) false false)
    (bind _asactivatable_object_parent_bp (cast `/Game/UGD_Game/Blueprints/activatable_object_parent_BP` (`self.target_obj`))
      (:`then`
        (`/Game/UGD_Game/Blueprints/activatable_object_parent_BP.Deactivate` _asactivatable_object_parent_bp))
      (:`CastFailed`
        (`KismetSystemLibrary.PrintString` "no target")))
    (else
      (`KismetSystemLibrary.PrintString` "wasnt a block"))))

(fn `Get colour`
  (switch `/Game/UGD_Game/Blueprints/Block_Stuff/BlockID_E` (`self.block_ID`)
    (:`NewEnumerator1`
      (`PrimitiveComponent.SetMaterial` (`self.Button face`) 0 null))
    (:`NewEnumerator2`
      (`PrimitiveComponent.SetMaterial` (`self.Button face`) 0 null))
    (:`NewEnumerator3`
      (`PrimitiveComponent.SetMaterial` (`self.Button face`) 0 null))
    (:`NewEnumerator4`
      (`PrimitiveComponent.SetMaterial` (`self.Button face`) 0 null))
    (:`NewEnumerator5`
      (`PrimitiveComponent.SetMaterial` (`self.Button face`) 0 null))
    (:`NewEnumerator6`
      (`PrimitiveComponent.SetMaterial` (`self.Button face`) 0 null))
    (:`NewEnumerator7`
      (`PrimitiveComponent.SetMaterial` (`self.Button face`) 0 null))
    (:`NewEnumerator8`
      (`PrimitiveComponent.SetMaterial` (`self.Button face`) 0 null))))

(fn `UserConstructionScript`)